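; MaxWell_BP is an actor that spins its MaxWell2SplitDiscoGrande70 component around local yaw.
; A timeline started at BeginPlay scales Speed against MaxSpeed, then enables input for player controller ID 0 when it finishes.
; While Spin is true, Tick applies the frame-time-scaled rotation, and the P key toggles Spin.
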(event EventBeginPlay
  (bind _newtrack_0 (Timeline|Timeline_0 Play)
    (:Update
      (Variables|Default|Setspeed (* _newtrack_0 (Variables|Default|GetMaxSpeed))))
    (:Finished
      (Input|EnableInput (Class|GameplayStatics|GetPlayerControllerfromID)))))

(event Collision|EventActorBeginOverlap
  (params (OtherActor :type Actor%20Object%20Reference)))

(event EventTick
  (params (DeltaSeconds :type Float%20%28single-precision%29))
  (if (Variables|Default|Getspin)
    (Transformation|AddLocalRotation (Variables|Default|GetMaxWell2Split_discoGrande_70) (Math|Rotator|MakeRotator 0.0 0.0 (* DeltaSeconds (Variables|Default|Getspeed))) false false)))

(event Input|KeyboardEvents|P
  (params (Key :type Key%20Structure :default "None"))
  (:Pressed
    (Variables|Default|Setspin (not (Variables|Default|Getspin)))))

(fn ConstructionScript)