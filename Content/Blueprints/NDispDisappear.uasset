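; NDispDisappear is an input-driven actor that shows or hides two referenced actors on key presses.
; BeginPlay enables input from the first player controller, with Z and X each bound to one of the actors.
; Both keys call a shared ToggleThis event, which toggles the root component's visibility along with its children and spawns a scaled-down chill explosion particle at its location.
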(event Custom|ToggleThis
  (params (Actor :type Scene%20Component%20Object%20Reference))
  (Rendering|ToggleVisibility Actor true)
  (Effects|SpawnEmitteratLocation "/Game/StarterContent/Particles/P_ChillExplosion.P_ChillExplosion" (Transformation|GetWorldLocation Actor) "0, 0, 0" "0.300000,0.300000,0.300000"))

(event EventBeginPlay
  (Input|EnableInput (Game|GetPlayerController 0)))

(event Collision|EventActorBeginOverlap
  (params (OtherActor :type Actor%20Object%20Reference)))

(event EventTick
  (params (DeltaSeconds :type Float%20%28single-precision%29)))

(event Input|KeyboardEvents|E
  (params (Key :type Key%20Structure :default "None")))

(event Input|KeyboardEvents|Z
  (params (Key :type Key%20Structure :default "None"))
  (:Pressed
    (CallFunction|ToggleThis (Variables|/Script/Engine.Actor|GetRootComponent (Variables|Default|GetActorToRespawn)))))

(event Input|KeyboardEvents|X
  (params (Key :type Key%20Structure :default "None"))
  (:Pressed
    (CallFunction|ToggleThis (Variables|/Script/Engine.Actor|GetRootComponent (Variables|Default|GetActorToRespawnToo)))))

(fn ConstructionScript)