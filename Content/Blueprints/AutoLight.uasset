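; AutoLight is an actor whose light component, Erwe, starts on and is toggled off and on with the E key.
; On BeginPlay it prints "Lights on", sets a very high intensity and enables input from the first player controller.
; Each E press drives a FlipFlop that alternates between zero and full intensity, with no overlap or distance check despite the name.
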(event EventBeginPlay
  (Development|PrintString "Lights on" true true "(R=0.000000,G=0.660000,B=1.000000,A=1.000000)" 5.0)
  (Rendering|Components|Light|SetIntensity (Variables|Default|Geterwe) 5e+05)
  (Input|EnableInput (Game|GetPlayerController 0)))

(event Collision|EventActorBeginOverlap
  (params (OtherActor :type Actor%20Object%20Reference)))

(event EventTick
  (params (DeltaSeconds :type Float%20%28single-precision%29)))

(event Input|KeyboardEvents|E
  (params (Key :type Key%20Structure :default "None"))
  (:Pressed
    (Utilities|FlowControl|FlipFlop
      (:A
        (Rendering|Components|Light|SetIntensity (Variables|Default|Geterwe) 0.0))
      (:B
        (Rendering|Components|Light|SetIntensity (Variables|Default|Geterwe) 5e+05)))))

(fn ConstructionScript)