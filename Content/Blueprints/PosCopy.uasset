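; PosCopy is an actor that mirrors another object's rotation onto its ObjCenter component while the player drives a spin input.
; Each tick, if ObjToCopyRot is valid and either the SpinThingL or SpinThingR axis passes a threshold, it copies that actor's world rotation.
; A DoOnce records StartRotation at the start of each spin, though nothing reads it.
; Player input is enabled on BeginPlay, and E toggles ObjCenter's visibility.
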(event EventBeginPlay
  (Input|EnableInput (Game|GetPlayerController 0)))

(event Collision|EventActorBeginOverlap
  (params (OtherActor :type Actor%20Object%20Reference)))

(event EventTick
  (params (DeltaSeconds :type Float%20%28single-precision%29))
  (Utilities|IsValid (Variables|Default|GetObjToCopyRot)
    (:Is%20Valid
      (if (or (> (Input|AxisValues|GetSpinThingL) 0.5) (> (Input|AxisValues|GetSpinThingR) 0.5))
        (Transformation|SetWorldRotation (Variables|Default|GetObjCenter) (Transformation|GetActorRotation (Variables|Default|GetObjToCopyRot)) false false)
        (Utilities|FlowControl|DoOnce false :!label _label
          (:Completed
            (Variables|Default|SetstartRotation (Transformation|GetActorRotation (Variables|Default|GetObjToCopyRot)))))
        (else
          (goto _label Reset))))))

(event Input|KeyboardEvents|E
  (params (Key :type Key%20Structure :default "None"))
  (:Pressed
    (Rendering|ToggleVisibility (Variables|Default|GetObjCenter) true)))

(fn ConstructionScript)