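; justSpiral_Blueprint is an actor that orients colored spiral components in proportion to Red, Green and Blue values.
; The construction script sums the three values, then yaws GreenSpiral by green's share of a full turn and BlueSpiral by the combined green and blue share.
; All placement happens at construction, as the BeginPlay, overlap and Tick events are empty.
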(event EventBeginPlay)

(event Collision|EventActorBeginOverlap
  (params (OtherActor :type Actor%20Object%20Reference)))

(event EventTick
  (params (DeltaSeconds :type Float%20%28single-precision%29)))

(fn ConstructionScript
  (bind _output_get (Variables|Default|Setsum (+ (Variables|Default|GetRed) (Variables|Default|GetGreen) (Variables|Default|GetBlue))))
  (Utilities|FlowControl|Sequence
    (:then_0
      (Transformation|SetRelativeRotation (Variables|Default|GetGreenSpiral) (Math|Rotator|MakeRotator 0.0 0.0 (* (/ (Variables|Default|GetGreen) _output_get) 3.6e+02)) false false))
    (:then_1
      (Transformation|SetRelativeRotation (Variables|Default|GetblueSpiral) (Math|Rotator|MakeRotator 0.0 0.0 (* (/ (+ (Variables|Default|GetBlue) (Variables|Default|GetGreen)) _output_get) 3.6e+02)) false false))))