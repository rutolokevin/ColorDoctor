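; Maxwell disc actor that rotates its large disc mesh around local yaw each tick at a rate set by Speed.
; BeginPlay creates dynamic materials for radial motion blur and a roughness-changing look, sharing the latter across three smaller disc meshes.
; A timeline meant to ramp speed, blur and material lerp from left/right spin inputs sits in a disconnected branch that never runs.
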(event EventBeginPlay
  (|CallParentFunction)
  (bind _returnvalue (Rendering|Material|CreateDynamicMaterialInstance (Variables|Default|GetBlurMesh) 0 "/Game/ExampleContent/Materials/Materials/MI_RadialMotionBlur.MI_RadialMotionBlur" "None" :!class /Script/Engine.PrimitiveComponent))
  (Variables|Default|SetblurMat _returnvalue)
  (Rendering|Material|SetScalarParameterValue (Variables|Default|GetBlurMat) "Angle" 0.0 :!class /Script/Engine.MaterialInstanceDynamic)
  (bind _returnvalue_2 (Rendering|Material|CreateDynamicMaterialInstance (Variables|Default|GetMaxWell2Split_disco3) 0 "/Game/ColorDoctor/Maxwell/ORM_MatRoughChanging.ORM_MatRoughChanging" "None" :!class /Script/Engine.PrimitiveComponent))
  (bind _output_get (Variables|Default|SetOrangeMat _returnvalue_2))
  (Rendering|Material|SetScalarParameterValue _output_get "Lerp" 0.0 :!class /Script/Engine.MaterialInstanceDynamic)
  (Rendering|Material|SetMaterial (Variables|Default|GetMaxWell2Split_disco4) 0 _output_get))

(event Collision|EventActorBeginOverlap
  (params (OtherActor :type Actor%20Object%20Reference))
  (|CallParentFunction OtherActor) ; This node is disabled and will not be called.\nDrag off pins to build functionality.
)

(event EventTick
  (params (DeltaSeconds :type Float%20%28single-precision%29))
  (|CallParentFunction DeltaSeconds)
  (Transformation|AddLocalRotation (Variables|Default|GetMaxWell2Split_discoGrande) (Math|Rotator|MakeRotator 0.0 0.0 (* DeltaSeconds (Variables|Default|Getspeed))) false false))

(fn ConstructionScript
  (|CallParentFunction))